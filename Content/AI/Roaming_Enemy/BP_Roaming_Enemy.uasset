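; Roaming AI enemy character that moves at walk or run speed and shoots projectiles at the player.
; Walk and Run events set the movement speed.
; Attack loops a rifle-firing animation, waits briefly, sets Attacking, spawns an enemy projectile at the weapon socket aimed at the player, then restores the animation blueprint.
; An unconnected line-trace hit check, including the only reset of Attacking, never runs.
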(event Custom|Walk
  (Variables|/Script/Engine.CharacterMovementComponent|SetMaxWalkSpeed (Variables|Character|GetCharacterMovement) 1.8e+02))

(event Custom|Run
  (Variables|/Script/Engine.CharacterMovementComponent|SetMaxWalkSpeed (Variables|Character|GetCharacterMovement) 3.5e+02))

(event Custom|Attack
  (bind _weapon (Variables|Default|GetWeapon))
  (bind _returnvalue (Transformation|GetSocketLocation _weapon "Weapon_Socket"))
  (bind (_x _y _z) (Math|Vector|BreakVector _returnvalue))
  (Components|Animation|PlayAnimation (Variables|Character|GetMesh) "/Game/Anims/EnemyAnims/Firing_Rifle.Firing_Rifle" true)
  (Utilities|FlowControl|Delay 1.5)
  (Variables|Default|SetAttacking true)
  (Game|SpawnActorfromClass "/Game/AI/BP_EnemyProjectile.BP_EnemyProjectile_C" (Math|Transform|MakeTransform (Math|Vector|MakeVector _x _y _z) (Math|Rotator|FindLookatRotation (Transformation|GetActorLocation) (Transformation|GetActorLocation (Game|GetPlayerCharacter 0))) "0.400000,0.400000,0.400000") "AlwaysSpawn" "MultiplyWithRoot" 0 0)
  (Components|Animation|SetAnimationMode (Variables|Character|GetMesh) "AnimationBlueprint"))

(fn ConstructionScript)