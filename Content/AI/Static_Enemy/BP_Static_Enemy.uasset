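; BP_Static_Enemy is an enemy that fires projectiles at the player when its Attack event is called.
; If the player is within range, it plays a rifle-firing animation, flags Attacking and waits briefly.
; It then spawns a BP_EnemyProjectile at the weapon socket, rotated toward the player, and restores Animation Blueprint mode.
; A disconnected line-trace damage check, containing the only Attacking reset, never runs.
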(event Custom|Attack
  (bind _returnvalue (Game|GetPlayerCharacter 0))
  (bind _weapon (Variables|Default|GetWeapon))
  (bind _returnvalue_2 (Transformation|GetSocketLocation _weapon "Weapon_Socket"))
  (bind (_x _y _z) (Math|Vector|BreakVector _returnvalue_2))
  (if (<= (Transformation|GetDistanceTo _returnvalue) 6e+02)
    (Components|Animation|PlayAnimation (Variables|Character|GetMesh) "/Game/Anims/EnemyAnims/Firing_Rifle.Firing_Rifle" false)
    (Variables|Default|SetAttacking true)
    (Utilities|FlowControl|Delay 1.5)
    (Game|SpawnActorfromClass "/Game/AI/BP_EnemyProjectile.BP_EnemyProjectile_C" (Math|Transform|MakeTransform (Math|Vector|MakeVector _x _y _z) (Math|Rotator|FindLookatRotation (Transformation|GetActorLocation) (Transformation|GetActorLocation _returnvalue)) "0.400000,0.400000,0.400000") "AlwaysSpawn" "MultiplyWithRoot" 0 0)
    (Components|Animation|SetAnimationMode (Variables|Character|GetMesh) "AnimationBlueprint")))

(event EventBeginPlay)

(event Collision|EventActorBeginOverlap
  (params (OtherActor :type Actor%20Object%20Reference)))

(event EventTick
  (params (DeltaSeconds :type Float%20%28single-precision%29)))

(fn ConstructionScript)